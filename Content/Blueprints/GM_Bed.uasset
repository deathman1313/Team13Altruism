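; GM_Bed is a wave manager, apparently a game mode, that runs ten enemy waves and then shows the win screen.
; PopulateMap loads each wave's small, medium and large enemy counts from DT_WaveDetails.
; A looping timer, paused at start and toggled by TimerStartStop, spawns a randomly chosen remaining enemy type at a random BP_SpawnPoint.
; When none remain to spawn or alive, the next tick advances the wave.
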(event Custom|ActivateSpawner
  (bind _spawnerlist (Variables|Default|GetSpawnerList))
  (if (> (Variables|Default|GetNumberOfEnemies) 0)
    (bind _enemychosen (CallFunction|ChooseEnemy))
    (Default|SpawnEnemy (Utilities|Array|Get(acopy) _spawnerlist (Math|Random|RandomIntegerinRange 0 (- (Utilities|Array|Length _spawnerlist) 1))) _enemychosen)
    (else
      (bind _outactors (Actor|GetAllActorsOfClass "/Game/Blueprints/AI/BP_EnemyAI.BP_EnemyAI_C")) ; Also inefficent, use same solution as before
      (if (<= (Utilities|Array|Length _outactors) 0)
        (bind _result (Math|Integer|IncrementInt (Variables|Default|GetWaveNumber))
          (:%20%20
            (if (<= _result 10)
              (CallFunction|PopulateMap _result)
              (else
                (bind _returnvalue (UserInterface|CreateWidget "/Game/Blueprints/UI/UI_WinScreen.UI_WinScreen_C" (Game|GetPlayerController 0)))
                (UserInterface|Viewport|AddtoViewport _returnvalue 0)))))))))

(event EventBeginPlay
  (bind _outactors (Actor|GetAllActorsOfClass "/Game/Blueprints/AI/BP_SpawnPoint.BP_SpawnPoint_C")) ; Inefficent, better to have all BP_SpawnPoint's add themselves to the array on begin play
  (Variables|Default|SetSpawnerList _outactors)
  (bind _returnvalue (Utilities|Time|SetTimerbyEvent (delegate Custom|ActivateSpawner) 3.0 true))
  (Variables|Default|SetTimerHandle _returnvalue)
  (CallFunction|TimerStartStop)
  (CallFunction|PopulateMap (Variables|Default|GetWaveNumber)))

(event EventTick
  (params (DeltaSeconds :type Float%20%28single-precision%29)))

(fn ConstructionScript)

(fn CalculateEnemyNumber
  (Variables|Default|SetNumberOfEnemies (- (* (Variables|Default|GetWaveNumber) 5) (* (Variables|Default|GetWaveNumber) 2))))

(fn PopulateMap
  (params (WaveNumber :type Integer))
  (bind _returnvalue (Utilities|GetDataTableRow "/Game/Blueprints/AI/DT_WaveDetails.DT_WaveDetails" (Utilities|String|StringToName (Utilities|String|ToString(Integer) WaveNumber)))
    (:then
      (bind _output_get (Variables|Default|SetEnemyList (Utilities|Map|MakeMap "/Game/Blueprints/AI/BP_EnemyAI_Small.BP_EnemyAI_Small_C" (.bp_enemyai_small _returnvalue) "/Game/Blueprints/AI/BP_EnemyAI_Medium.BP_EnemyAI_Medium_C" (.bp_enemyai_medium _returnvalue) "/Game/Blueprints/AI/BP_EnemyAI_Large.BP_EnemyAI_Large_C" (.bp_enemyai_large _returnvalue))))
      (bind _values (Utilities|Map|Values _output_get))
      (for _array_element _values
        (Variables|Default|SetNumberOfEnemies (+ _array_element (Variables|Default|GetNumberOfEnemies)))))))

(fn ChooseEnemy
  (bind _keys (Utilities|Map|Keys (Variables|Default|GetEnemyList) :!label _label))
  (bind _output_get (LocalVariables|SetChosenEnemy (Utilities|Array|Get(acopy) _keys (Math|Random|RandomInteger (Utilities|Array|Length _keys)))))
  (LocalVariables|SetEnemy%20Number (.Value (Utilities|Map|Find (Variables|Default|GetEnemyList) _output_get)))
  (if (> (.Value (Utilities|Map|Find (Variables|Default|GetEnemyList) _output_get)) 0)
    (Utilities|Map|Add (Variables|Default|GetEnemyList) (LocalVariables|GetChosenEnemy) (- (LocalVariables|GetEnemy%20Number) 1))
    (Variables|Default|SetNumberOfEnemies (- (Variables|Default|GetNumberOfEnemies) 1))
    (return (LocalVariables|GetChosenEnemy))
    (else
      (goto _label))))

(fn TimerStartStop
  (bind _timerhandle (Variables|Default|GetTimerHandle))
  (if (Class|KismetSystemLibrary|IsTimerPausedHandle _timerhandle)
    (Utilities|Time|UnpauseTimerbyHandle _timerhandle)
    (else
      (Utilities|Time|PauseTimerbyHandle _timerhandle))))