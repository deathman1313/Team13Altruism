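; BP_Pickup is a typed pickup that adds to a Teddy character's stock of a tower weapon.
; On BeginPlay it sets its static mesh by looking up PickupType in a Meshes map.
; When BP_Teddy overlaps the sphere, it disables further overlaps, adds Amount to the WeaponTypes entry whose Tower matches PickupType, then destroys itself.
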(event OnComponentBeginOverlap(Sphere)
  (params (OverlappedComponent :type Primitive%20Component%20Object%20Reference) (OtherActor :type Actor%20Object%20Reference) (OtherComp :type Primitive%20Component%20Object%20Reference) (OtherBodyIndex :type Integer) (bFromSweep :type Boolean) (SweepResult :type Hit%20Result%20Structure%20%28by%20ref%29))
  (bind _asbp_teddy (Utilities|Casting|CastToBP_Teddy OtherActor))
  (Variables|/Script/Engine.PrimitiveComponent|SetbGenerateOverlapEvents (Variables|Default|GetSphere) false)
  (bind (_array_element _array_index) (Utilities|Array|ForEachLoopwithBreak (Variables|/Game/Blueprints/BP_Teddy.BP_Teddy_C|GetWeaponTypes _asbp_teddy) :!label _label)
    (:LoopBody
      (if (== (.tower _array_element) (Variables|Default|GetPickupType))
        (Utilities|Array|SetArrayElem (Variables|/Game/Blueprints/BP_Teddy.BP_Teddy_C|GetWeaponTypes _asbp_teddy) _array_index (Utilities|Struct|MakeST_TowerSelection (.tower _array_element) (.mesh _array_element) 0 (+ (.amount _array_element) (Variables|Default|GetAmount))))
        (goto _label Break)))
    (:Completed
      (Actor|DestroyActor))))

(event EventBeginPlay
  (Components|StaticMesh|SetStaticMesh (Variables|Default|GetStaticMesh) (.Value (Utilities|Map|Find (Variables|Default|GetMeshes) (Variables|Default|GetPickupType)))))

(event Collision|EventActorBeginOverlap
  (params (OtherActor :type Actor%20Object%20Reference)))

(event EventTick
  (params (DeltaSeconds :type Float%20%28single-precision%29)))

(fn ConstructionScript)