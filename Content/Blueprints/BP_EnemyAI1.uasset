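; Enemy AI pawn that walks a one-way route through five locations on BeginPlay and attacks BP_Teddy, the player character, when PawnSensing spots it.
; ChasePlayer uses AI MoveTo to reach the target, applies damage, then re-calls itself after a short delay while sensing stays enabled.
; The player's death event is bound to ResetAI, which disables sensing and sends the enemy to the route's final location.
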(event OnSeePawn(PawnSensing)
  (params (Pawn :type Pawn%20Object%20Reference))
  (bind _asbp_teddy (Utilities|Casting|CastToBP_Teddy Pawn))
  (CallFunction|ChasePlayer _asbp_teddy))

(event Custom|ChasePlayer
  (params (PlayerToChase :type Pawn%20Object%20Reference))
  (if (Variables|/Script/AIModule.PawnSensingComponent|GetbEnableSensingUpdates (Variables|Default|GetPawnSensing))
    (AI|AIMoveTo self "0, 0, 0" PlayerToChase 5.0 false
      (:OnSuccess
        (Game|Damage|ApplyDamage PlayerToChase (Variables|Default|GetDamage) 0 0)
        (Utilities|FlowControl|Delay 1.0)
        (CallFunction|ChasePlayer PlayerToChase)))))

(event Custom|Reset%20AI
  (Class|PawnSensingComponent|SetSensingUpdatesEnabled (Variables|Default|GetPawnSensing) false)
  (AI|AIMoveTo self (Variables|Default|GetLocation%205) 0 5.0 false))

(event EventBeginPlay
  (bind _self self)
  (bind _asbp_teddy (Utilities|Casting|CastToBP_Teddy (Game|GetPlayerCharacter 0)))
  (EventDispatchers|BindEventtoPlayerDied _asbp_teddy (delegate Custom|Reset%20AI))
  (AI|AIMoveTo _self (Variables|Default|GetLocation%201) 0 5.0 false
    (:OnSuccess
      (AI|AIMoveTo _self (Variables|Default|GetLocation%202) 0 5.0 false
        (:OnSuccess
          (AI|AIMoveTo _self (Variables|Default|GetLocation%203) 0 5.0 false
            (:OnSuccess
              (AI|AIMoveTo _self (Variables|Default|GetLocation%204) 0 5.0 false
                (:OnSuccess
                  (AI|AIMoveTo _self (Variables|Default|GetLocation%205) 0 5.0 false))))))))))

(event Collision|EventActorBeginOverlap
  (params (OtherActor :type Actor%20Object%20Reference)))

(event EventTick
  (params (DeltaSeconds :type Float%20%28single-precision%29)))

(fn ConstructionScript)