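; Player character for a point-and-click tower-placement game, handling movement, tower selection, health, pausing and score.
; A decal follows the mouse trace, and holding Move repeatedly calls SimpleMoveToLocation toward it.
; A looping timer sends hover/unhover messages to grid actors under the cursor, while Interact passes them the scroll-selected tower if any remain.
; Highscore loads from SG_Highscore before HUD creation and saves whenever the score beats it.
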(event Custom|GridHover
  (bind _returnvalue (Game|GetPlayerController 0))
  (bind _array (Utilities|Array|MakeArray "ObjectTypeQuery8"))
  (bind _hitresult (Class|PlayerController|GetHitResultUnderCursorforObjects _returnvalue _array false))
  (bind (_bblockinghit _binitialoverlap _time _distance _location _impactpoint _normal _impactnormal _physmat _hitactor) (Collision|BreakHitResult _hitresult))
  ;[1 1 1] Interact with Grid
  (Class|BPIGridInteraction|GridHovered(Message) _hitactor (.mesh (Utilities|Array|Get(acopy) (Variables|Default|GetWeaponTypes) (Variables|Default|GetSelectedWeapon))) _location)
  (if (!= (Variables|Default|GetPrevLookAt) _hitactor)
    (Class|BPIGridInteraction|GridUnhovered(Message) (Variables|Default|GetPrevLookAt))
    (Variables|Default|SetPrevLookAt _hitactor)))

(event Custom|MoveToCursor
  (bind _returnvalue (Game|GetPlayerController 0))
  ;[1 1 1] Point and Click Movement
  (AI|Navigation|SimpleMovetoLocation _returnvalue (.Location (Collision|BreakHitResult (.HitResult (Class|PlayerController|GetHitResultUnderCursorforObjects _returnvalue (Utilities|Array|MakeArray "ObjectTypeQuery1") false))))))

(event EventBeginPlay
  (Variables|/Script/Engine.PlayerController|SetbShowMouseCursor (Game|GetPlayerController 0) true)
  ;[1 1 1] Create Cursor
  (bind _returnvalue (Game|SpawnActorfromClass "/Script/Engine.DecalActor" (Math|Transform|MakeTransform "0, 0, 0" "0, 0, 0" "0.100000,0.100000,0.100000") "Undefined" 0 0))
  (Variables|Default|SetCursor _returnvalue)
  (Utilities|Time|SetTimerbyEvent (delegate Custom|GridHover) 0.1 true)
  ;[1 1 1] Load Highscore
  (bind _returnvalue_2 (SaveGame|DoesSaveGameExist (Variables|Default|GetSlotName)))
  (if _returnvalue_2
    (bind _returnvalue_3 (SaveGame|LoadGamefromSlot (Variables|Default|GetSlotName)))
    (bind _assg_highscore (Utilities|Casting|CastToSG_Highscore _returnvalue_3))
    (Variables|Default|SetHighscore (Variables|/Game/Blueprints/SG_Highscore.SG_Highscore_C|GetHighscore _assg_highscore)))
  ;[1 1 1] Create Hud
  (bind _returnvalue_4 (UserInterface|CreateWidget "/Game/Blueprints/UI/UI_Hud.UI_Hud_C" (Game|GetPlayerController 0)))
  (bind _output_get (Variables|Default|SetHUD _returnvalue_4))
  (UserInterface|Viewport|AddtoViewport _output_get 0))

(event Game|Damage|EventAnyDamage
  (params (Damage :type Float%20%28single-precision%29) (DamageType :type Damage%20Type%20Object%20Reference) (InstigatedBy :type Controller%20Object%20Reference) (DamageCauser :type Actor%20Object%20Reference))
  ;[1 1 1] Damage
  (bind _output_get (Variables|Default|SetCurrentHealth (- (Variables|Default|GetCurrentHealth) Damage)))
  (if (<= _output_get 0.0)
    (Default|CallPlayerDied)))

(event EventTick
  (params (DeltaSeconds :type Float%20%28single-precision%29))
  ;[1 1 1] Point and Click Movement
  (Transformation|SetWorldLocation (Variables|/Script/Engine.Actor|GetRootComponent (Variables|Default|GetCursor)) (.Location (Collision|BreakHitResult (.HitResult (Class|PlayerController|GetHitResultUnderCursorforObjects (Game|GetPlayerController 0) (Utilities|Array|MakeArray "ObjectTypeQuery1") false)))) false false))

(event Input|ActionEvents|InputActionPause
  (params (Key :type Key%20Structure))
  ;[1 1 1] Pause the game
  (:Pressed
    (CallFunction|PauseGame)))

(event Input|ActionEvents|InputActionInteract
  (params (Key :type Key%20Structure))
  (bind _returnvalue (Game|GetPlayerController 0))
  (bind _array (Utilities|Array|MakeArray "ObjectTypeQuery8"))
  (bind _weapontypes (Variables|Default|GetWeaponTypes))
  (bind _selectedweapon (Variables|Default|GetSelectedWeapon))
  (bind _hitresult (Class|PlayerController|GetHitResultUnderCursorforObjects _returnvalue _array false))
  (bind _output (Utilities|Array|Get(acopy) _weapontypes _selectedweapon))
  (bind (_bblockinghit _binitialoverlap _time _distance _location _impactpoint _normal _impactnormal _physmat _hitactor) (Collision|BreakHitResult _hitresult))
  ;[1 1 1] Interact with Grid
  (:Pressed
    (if (> (.amount _output) 0)
      (Class|BPIGridInteraction|GridInteracted(Message) _hitactor (.tower _output) _location)
      (Variables|Default|SetWeaponToRemove (Variables|Default|GetSelectedWeapon)))))

(event Input|ActionEvents|InputActionMove
  (params (Key :type Key%20Structure))
  ;[1 1 1] Point and Click Movement
  (:Pressed
    (bind _returnvalue (Utilities|Time|SetTimerbyEvent (delegate Custom|MoveToCursor) 0.01 true)))
  (:Released
    (Utilities|Time|ClearandInvalidateTimerbyHandle _returnvalue)))

(event Input|ActionEvents|InputActionStartandstoptimer
  (params (Key :type Key%20Structure))
  ;[1 1 1] Timer (WIP)
  (:Pressed
    (bind _asgm_bed (Utilities|Casting|CastToGM_Bed (Game|GetGameMode)))
    (Default|TimerStartStop _asgm_bed)))

(event Input|AxisEvents|InputAxisScroll
  (params (AxisValue :type Float%20%28single-precision%29))
  ;[1 1 1] Select Tower
  (if (!= AxisValue 0.0)
    (Variables|Default|SetSelectedWeapon (Math|Integer|Clamp(Integer) (+ (Math|Float|Truncate AxisValue) (Variables|Default|GetSelectedWeapon)) 0 (Utilities|Array|LastIndex (Variables|Default|GetWeaponTypes))))))

(fn ConstructionScript)

(fn PauseGame
  (Game|SetGamePaused true)
  (Utilities|IsValid (Variables|Default|GetPauseMenu)
    (:Is%20Valid
      _)
    (:Is%20Not%20Valid
      (bind _returnvalue (UserInterface|CreateWidget "/Game/Blueprints/UI/Menus/UI_PauseMenu.UI_PauseMenu_C" (Game|GetPlayerController 0)))
      (Variables|Default|SetPauseMenu _returnvalue)))
  (UserInterface|Viewport|AddtoViewport (Variables|Default|GetPauseMenu) 0)
  (Input|SetInputModeUIOnly (Game|GetPlayerController 0) (Variables|Default|GetPauseMenu) "DoNotLock"))

(fn UnpauseGame
  (params (Menu :type UI%20Pause%20Menu%20Object%20Reference))
  (Game|SetGamePaused false)
  (Widget|RemovefromParent Menu)
  (Input|SetInputModeGameandUI (Game|GetPlayerController 0) 0 "DoNotLock" false))

(fn RemoveWeapon
  (Math|Integer|DecrementInt (.amount (Utilities|Array|Get(acopy) (Variables|Default|GetWeaponTypes) (Variables|Default|GetWeaponToRemove)))))

(fn IncreaseScore
  (params (Amount :type Integer))
  (bind _output_get (Variables|Default|SetScore (+ (Variables|Default|GetScore) Amount)))
  (if (> _output_get (Variables|Default|GetHighscore))
    (Variables|Default|SetHighscore (Variables|Default|GetScore))
    (bind _returnvalue (SaveGame|DoesSaveGameExist (Variables|Default|GetSlotName)))
    (if _returnvalue
      (bind _returnvalue_2 (SaveGame|LoadGamefromSlot))
      (Variables|Default|SetSaverSubClass _returnvalue_2)
      (else
        (bind _returnvalue_3 (SaveGame|CreateSaveGameObject))
        (Variables|Default|SetSaverSubClass _returnvalue_3)))
    (bind _assg_highscore (Utilities|Casting|CastToSG_Highscore (Variables|Default|GetSaverSubClass)))
    (Variables|/Game/Blueprints/SG_Highscore.SG_Highscore_C|SetHighscore _assg_highscore (Variables|Default|GetHighscore))
    (SaveGame|SaveGametoSlot (Variables|Default|GetSaverSubClass) (Variables|Default|GetSlotName))))