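; BP_EnemyAI is an enemy that walks to an end location and destroys itself on arrival.
; Damage lowers its health, and at zero it adds its point value to the BP_Teddy player's score and is destroyed.
; It binds to Teddy's PlayerDied event, which turns off pawn sensing, reissues the move to the end location and shows the lose screen when that move succeeds.
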(event Custom|Reset%20AI
  ;[1 1 1] If player died
  (Class|PawnSensingComponent|SetSensingUpdatesEnabled (Variables|Default|GetPawnSensing) false)
  (AI|AIMoveTo self (Variables|Default|GetLocation%20End) 0 5.0 false
    (:OnSuccess
      (bind _returnvalue (UserInterface|CreateWidget "/Game/Blueprints/UI/UI_LoseScreen.UI_LoseScreen_C"))
      (UserInterface|Viewport|AddtoViewport _returnvalue 0))))

(event EventBeginPlay
  ;[1 1 1] If player died
  (bind _asbp_teddy (Utilities|Casting|CastToBP_Teddy (Game|GetPlayerCharacter 0)))
  (EventDispatchers|BindEventtoPlayerDied _asbp_teddy (delegate Custom|Reset%20AI))
  ;[1 1 1] Move to Point
  (AI|AIMoveTo self (Variables|Default|GetLocation%20End) 0 5.0 false
    (:OnSuccess
      (Actor|DestroyActor))))

(event Collision|EventActorBeginOverlap
  (params (OtherActor :type Actor%20Object%20Reference)))

(event EventTick
  (params (DeltaSeconds :type Float%20%28single-precision%29)))

(event Game|Damage|EventAnyDamage
  (params (Damage :type Float%20%28single-precision%29) (DamageType :type Damage%20Type%20Object%20Reference) (InstigatedBy :type Controller%20Object%20Reference) (DamageCauser :type Actor%20Object%20Reference))
  ;[1 1 1] AI Death
  (bind _output_get (Variables|Default|SetHealth (- (Variables|Default|GetHealth) Damage)))
  (if (<= _output_get 0.0)
    (Default|IncreaseScore (.AsBP%20Teddy (Utilities|Casting|CastToBP_Teddy (Game|GetPlayerCharacter 0))) (Variables|Default|GetPointValue))
    (Actor|DestroyActor)))

(fn ConstructionScript)