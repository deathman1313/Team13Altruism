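; BP_Grid is a placement grid on a plane where the player previews and places weapons.
; Hovering snaps a hologram mesh to empty cells, turning red while it overlaps actors.
; Interacting with a valid cell positions a trigger box and sends the player there.
; When BP_Teddy enters the box, the weapon spawns, is recorded in GridContent, and is removed from the player, whose movement stops.
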(event OnComponentBeginOverlap(PreviewMesh)
  (params (OverlappedComponent :type Primitive%20Component%20Object%20Reference) (OtherActor :type Actor%20Object%20Reference) (OtherComp :type Primitive%20Component%20Object%20Reference) (OtherBodyIndex :type Integer) (bFromSweep :type Boolean) (SweepResult :type Hit%20Result%20Structure%20%28by%20ref%29))
  (bind _overlappingactors (Variables|Default|GetOverlappingActors))
  ;[1 1 1] Determine Valid Spawn
  (Utilities|Array|Add _overlappingactors OtherActor)
  (Variables|Default|SetIsValidSpawn (== (Utilities|Array|Length _overlappingactors) 0))
  (CallFunction|SetMeshMaterial))

(event OnComponentEndOverlap(PreviewMesh)
  (params (OverlappedComponent :type Primitive%20Component%20Object%20Reference) (OtherActor :type Actor%20Object%20Reference) (OtherComp :type Primitive%20Component%20Object%20Reference) (OtherBodyIndex :type Integer))
  (bind _overlappingactors (Variables|Default|GetOverlappingActors))
  ;[1 1 1] Determine Valid Spawn
  (Utilities|Array|RemoveItem _overlappingactors OtherActor)
  (Variables|Default|SetIsValidSpawn (== (Utilities|Array|Length _overlappingactors) 0))
  (CallFunction|SetMeshMaterial))

(event OnComponentBeginOverlap(SpawnRadius)
  (params (OverlappedComponent :type Primitive%20Component%20Object%20Reference) (OtherActor :type Actor%20Object%20Reference) (OtherComp :type Primitive%20Component%20Object%20Reference) (OtherBodyIndex :type Integer) (bFromSweep :type Boolean) (SweepResult :type Hit%20Result%20Structure%20%28by%20ref%29))
  (bind _spawnradius (Variables|Default|GetSpawnRadius))
  ;[1 1 1] Spawn Weapon
  (Utilities|Casting|CastToBP_Teddy OtherActor)
  (Variables|/Script/Engine.PrimitiveComponent|SetbGenerateOverlapEvents _spawnradius false)
  (bind _returnvalue (Game|SpawnActorfromClass (Variables|Default|GetWeaponToSpawn) (Math|Transform|MakeTransform (Transformation|GetWorldLocation _spawnradius) "0,-90.000000, 0" "1,1,1") "AlwaysSpawn" 0 self 0))
  (if (Utilities|IsValid _returnvalue)
    (bind _asbp_teddy (Utilities|Casting|CastToBP_Teddy (Game|Player|GetPlayerPawn 0)))
    (Default|RemoveWeapon _asbp_teddy)
    (Transformation|SetWorldLocation (Variables|/Game/Blueprints/Towers/BP_Weapon.BP_Weapon_C|GetDefaultSceneRoot _returnvalue) (Math|Vector|MakeVector (.x (Transformation|GetWorldLocation (Variables|/Game/Blueprints/Towers/BP_Weapon.BP_Weapon_C|GetDefaultSceneRoot _returnvalue))) (.y (Transformation|GetWorldLocation (Variables|/Game/Blueprints/Towers/BP_Weapon.BP_Weapon_C|GetDefaultSceneRoot _returnvalue))) (- (.z (Transformation|GetWorldLocation (Variables|/Game/Blueprints/Towers/BP_Weapon.BP_Weapon_C|GetDefaultSceneRoot _returnvalue))) (.z (.Min (Components|StaticMesh|GetLocalBounds (Variables|/Game/Blueprints/Towers/BP_Weapon.BP_Weapon_C|GetStaticMesh _returnvalue)))))) false true)
    (Utilities|Array|SetArrayElem (Variables|Default|GetGridContent) (Variables|Default|GetIndexToSpawnIn) _returnvalue true)
    (Rendering|SetVisibility (Variables|Default|GetPreviewMesh) false true)
    (AI|Navigation|StopMovement (Game|GetPlayerController 0))))

(event EventBeginPlay
  (Components|Box|SetBoxExtent (Variables|Default|GetSpawnRadius) (Math|Vector|MakeVector (/ 7e+01 (Math|Conversions|ToFloat(Integer) (Variables|Default|GetGridRows))) (/ 7e+01 (Math|Conversions|ToFloat(Integer) (Variables|Default|GetGridColumns))) 1e+01) true))

(event EventGridHovered
  (params (Mesh :type Static%20Mesh%20Object%20Reference) (Position :type Vector :default "0, 0, 0"))
  (bind _previewmesh (Variables|Default|GetPreviewMesh))
  ;[1 1 1] Weapon Preview
  (if (!= Mesh (Variables|/Script/Engine.StaticMeshComponent|GetStaticMesh _previewmesh))
    (Components|StaticMesh|SetStaticMesh _previewmesh Mesh)
    (for (_ _array_index) (Rendering|Material|GetMaterials _previewmesh)
      (Rendering|Material|SetMaterial _previewmesh _array_index (select (Variables|Default|GetIsValidSpawn) "/Game/Materials/MI_HologramBlue.MI_HologramBlue" "/Game/Materials/MI_HologramRed.MI_HologramRed"))))
  (bind (_index _index2d) (CallFunction|WorldtoIndex Position))
  (Variables|Default|SetSelectedSpace _index)
  (if (not (Utilities|IsValid (Utilities|Array|Get(acopy) (Variables|Default|GetGridContent) _index)))
    (bind _location (CallFunction|IndextoSpaceCenter _index2d))
    (Transformation|SetWorldLocation _previewmesh (Math|Vector|MakeVector (.x _location) (.y _location) (- (.z _location) (.z (.Min (Components|StaticMesh|GetLocalBounds (Variables|Default|GetPreviewMesh)))))) false true)
    (Rendering|SetVisibility _previewmesh true true)
    (else
      (CallFunction|GridUnhovered))))

(event EventGridUnhovered
  ;[1 1 1] Weapon Preview
  (Rendering|SetVisibility (Variables|Default|GetPreviewMesh) false true))

(event EventGridInteracted
  (params (Weapon :type BP%20Weapon%20Class%20Reference) (Position :type Vector :default "0, 0, 0"))
  (bind _spawnradius (Variables|Default|GetSpawnRadius))
  ;[1 1 1] Position Spawn Radius
  (bind (_index _index2d) (CallFunction|WorldtoIndex Position))
  (if (and (not (Utilities|IsValid (Utilities|Array|Get(acopy) (Variables|Default|GetGridContent) _index))) (Variables|Default|GetIsValidSpawn))
    (bind _location (CallFunction|IndextoSpaceCenter _index2d))
    (Transformation|SetWorldLocation _spawnradius _location false true)
    (Variables|Default|SetWeaponToSpawn Weapon)
    (Variables|Default|SetIndexToSpawnIn _index)
    (Variables|/Script/Engine.PrimitiveComponent|SetbGenerateOverlapEvents _spawnradius true)
    (AI|Navigation|SimpleMovetoLocation (Game|GetPlayerController 0) _location)))

(fn ConstructionScript)

(fn WorldtoIndex
  (params (Location :type Vector))
  (bind _plane (Variables|Default|GetPlane))
  (bind _gridrows (Variables|Default|GetGridRows))
  (bind _gridcolumns (Variables|Default|GetGridColumns))
  (bind _returnvalue (Transformation|GetWorldScale _plane))
  (bind _returnvalue_2 (Math|Conversions|ToFloat(Integer) _gridrows))
  (bind _returnvalue_3 (Math|Conversions|ToFloat(Integer) _gridcolumns))
  (bind _returnvalue_4 (Transformation|GetWorldLocation _plane))
  (bind _returnvalue_5 (- _returnvalue_4 Location))
  (bind _returnvalue_6 (* _returnvalue 50))
  (bind _returnvalue_7 (* _returnvalue 100))
  (bind _returnvalue_8 (- (Math|Vector|MakeVector (.x _returnvalue_6) (.y _returnvalue_6) 0.0) _returnvalue_5))
  (bind _returnvalue_9 (/ (.x _returnvalue_7) _returnvalue_2))
  (bind _returnvalue_10 (/ (.y _returnvalue_7) _returnvalue_3))
  (bind _returnvalue_11 (/ (.x _returnvalue_8) _returnvalue_9))
  (bind _returnvalue_12 (/ (.y _returnvalue_8) _returnvalue_10))
  (bind _returnvalue_13 (Math|Float|Ceil _returnvalue_12))
  (bind _returnvalue_14 (Math|Float|Ceil _returnvalue_11))
  (return (- (+ _returnvalue_14 (* (- _returnvalue_13 1) (Variables|Default|GetGridColumns))) 1) (Utilities|Struct|MakeIntPoint _returnvalue_14 _returnvalue_13)))

(fn IndextoSpaceCenter
  (params (Index2D :type Int%20Point%20Structure))
  (bind (_x _y) (Utilities|Struct|BreakIntPoint Index2D))
  (bind _plane (Variables|Default|GetPlane))
  (bind _gridrows (Variables|Default|GetGridRows))
  (bind _gridcolumns (Variables|Default|GetGridColumns))
  (bind _returnvalue (Transformation|GetWorldLocation _plane))
  (bind _returnvalue_2 (Transformation|GetWorldScale _plane))
  (bind _returnvalue_3 (Math|Conversions|ToFloat(Integer) _gridrows))
  (bind _returnvalue_4 (Math|Conversions|ToFloat(Integer) _gridcolumns))
  (bind _returnvalue_5 (* _returnvalue_2 100))
  (bind _returnvalue_6 (/ (.x _returnvalue_5) _returnvalue_3))
  (bind _returnvalue_7 (/ (.y _returnvalue_5) _returnvalue_4))
  (return (Math|Vector|MakeVector (+ (- (+ (* (- _x 1) _returnvalue_6) (/ _returnvalue_6 2.0)) (/ (.x _returnvalue_5) 2.0)) (.x _returnvalue)) (+ (- (+ (* (- _y 1) _returnvalue_7) (/ _returnvalue_7 2.0)) (/ (.y _returnvalue_5) 2.0)) (.y _returnvalue)) (.z _returnvalue))))

(fn GetBoxSize
  (bind _plane (Variables|Default|GetPlane))
  (bind _returnvalue (Transformation|GetWorldScale _plane))
  (bind _returnvalue_2 (* _returnvalue 100))
  (return (Math|Vector2D|MakeVector2D (/ (.x _returnvalue_2) (Math|Conversions|ToFloat(Integer) (Variables|Default|GetGridRows))) (/ (.y _returnvalue_2) (Math|Conversions|ToFloat(Integer) (Variables|Default|GetGridColumns))))))

(fn SetMeshMaterial
  (bind _previewmesh (Variables|Default|GetPreviewMesh))
  (for (_ _array_index) (Rendering|Material|GetMaterials _previewmesh)
    (Rendering|Material|SetMaterial _previewmesh _array_index (select (Variables|Default|GetIsValidSpawn) "/Game/Materials/MI_HologramBlue.MI_HologramBlue" "/Game/Materials/MI_HologramRed.MI_HologramRed"))))