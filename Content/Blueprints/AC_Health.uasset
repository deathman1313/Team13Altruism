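; AC_Health is an actor component that tracks an owner's health and handles damage, healing and death.
; On BeginPlay it fills Health to MaxHealth and binds TakeDamage to the owner's OnTakeAnyDamage event.
; Damage subtracts from Health and destroys the owner at zero or below, while Heal adds health clamped to MaxHealth.
; DamageTaken, Healed and Killed dispatchers let other Blueprints hook custom responses.
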(event Custom|TakeDamage
  (params (DamagedActor :type Actor%20Object%20Reference) (Damage :type Float%20%28single-precision%29) (DamageType :type Damage%20Type%20Object%20Reference) (InstigatedBy :type Controller%20Object%20Reference) (DamageCauser :type Actor%20Object%20Reference))
  ;[1 1 1] Lower Health
  (Default|CallDamageTaken) ; Bind to for custom damage events
  (bind _output_get (Variables|Default|SetHealth (- (Variables|Default|GetHealth) Damage)))
  ;[1 1 1] Destroy if Killed
  (if (<= _output_get 0.0)
    (Default|CallKilled) ; Bind to for custom kill events
    (Actor|DestroyActor (Components|GetOwner))))

(event Custom|Heal
  (params (HealthGained :type Float%20%28single-precision%29))
  ;[1 1 1] Add Health
  (Default|CallHealed) ; Bind to for custom heal events
  (Variables|Default|SetHealth (Math|Float|Clamp(Float) (+ (Variables|Default|GetHealth) HealthGained) 0.0 (Variables|Default|GetMaxHealth))))

(event EventBeginPlay
  (Variables|Default|SetHealth (Variables|Default|GetMaxHealth))
  (EventDispatchers|BindEventtoOnTakeAnyDamage (Components|GetOwner) (delegate Custom|TakeDamage)))