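; BP_Block is a block actor in the Towers set that sizes itself to fit a grid box.
; On BeginPlay it runs the parent logic, then, if GridRef is valid, sets a uniform scale from the smaller of the grid box's X and Y dimensions.
; The construction script only calls its parent, and the overlap and Tick events are disabled stubs.
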(event EventBeginPlay
  (bind _gridref (Variables|Default|GetGridRef))
  ;[1 1 1] Set Box Size to Grid
  (|CallParentFunction)
  (if (Utilities|IsValid _gridref)
    (bind _dimentions (Default|GetBoxSize _gridref))
    (Transformation|SetActorScale3D (Math|Conversions|ToVector(Float) (Math|Float|Min(Float) (.x _dimentions) (.y _dimentions))))))

(event Collision|EventActorBeginOverlap
  (params (OtherActor :type Actor%20Object%20Reference))
  (|CallParentFunction OtherActor) ; This node is disabled and will not be called.\nDrag off pins to build functionality.
)

(event EventTick
  (params (DeltaSeconds :type Float%20%28single-precision%29))
  (|CallParentFunction DeltaSeconds) ; This node is disabled and will not be called.\nDrag off pins to build functionality.
)

(fn ConstructionScript
  (|CallParentFunction))