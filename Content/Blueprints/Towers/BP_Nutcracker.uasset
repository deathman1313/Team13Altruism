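; Nutcracker tower that periodically damages a single enemy within its range.
; When ready, Tick scans overlapping BP_EnemyAI actors and replaces the stored target with any that is closer to the tower mesh.
; A timeline turns the whole tower toward that target along the shortest path, then applies damage.
; A timer re-enables attacking after a fixed cooldown that starts once the hit lands.
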(event Custom|SetCanFire
  ;[1 1 1] Damage Target
  (Variables|Default|SetCanAttack true))

(event EventBeginPlay
  (|CallParentFunction))

(event Collision|EventActorBeginOverlap
  (params (OtherActor :type Actor%20Object%20Reference))
  (|CallParentFunction OtherActor) ; This node is disabled and will not be called.\nDrag off pins to build functionality.
)

(event EventTick
  (params (DeltaSeconds :type Float%20%28single-precision%29))
  (bind _staticmesh (Variables|Default|GetStaticMesh))
  (bind _defaultsceneroot (Variables|Default|GetDefaultSceneRoot))
  (bind _range (Variables|Default|GetRange))
  (bind _overlappingactors (Collision|GetOverlappingActors _range "/Game/Blueprints/AI/BP_EnemyAI.BP_EnemyAI_C" :!class /Script/Engine.PrimitiveComponent))
  (bind _returnvalue (Transformation|GetWorldLocation _staticmesh))
  (|CallParentFunction DeltaSeconds)
  (if (and (Variables|Default|GetCanAttack) (> (Utilities|Array|Length _overlappingactors) 0))
    (Variables|Default|SetCanAttack false)
    ;[1 1 1] Select Target
    (for _array_element _overlappingactors
      (if (< (Math|Vector|Distance(Vector) (Transformation|GetActorLocation _array_element) _returnvalue) (Math|Vector|Distance(Vector) _returnvalue (Transformation|GetActorLocation (Variables|Default|GetAttackingActor))))
        (bind _asbp_enemy_ai (Utilities|Casting|CastToBP_EnemyAI _array_element))
        (Variables|Default|SetAttackingActor _asbp_enemy_ai)))
    ;[1 1 1] Rotate to Target
    (if (Utilities|IsValid (Variables|Default|GetAttackingActor))
      (bind _output_get (Variables|Default|SetStartRotation (Transformation|GetWorldRotation _defaultsceneroot)))
      (bind _alpha (Timeline|RotateToTarget PlayFromStart)
        (:Update
          (Transformation|SetWorldRotation (Variables|Default|GetDefaultSceneRoot) (Math|Rotator|Lerp(Rotator) _output_get (Math|Rotator|FindLookatRotation (Transformation|GetWorldLocation _defaultsceneroot) (Transformation|GetActorLocation (Variables|Default|GetAttackingActor))) _alpha true) false false))
        (:Finished
          ;[1 1 1] Damage Target
          (Game|Damage|ApplyDamage (Variables|Default|GetAttackingActor) (Variables|Default|GetDamage) 0 self "/Script/Engine.DamageType")
          (Utilities|Time|SetTimerbyEvent (delegate Custom|SetCanFire) 5.0))))))

(fn ConstructionScript
  (|CallParentFunction))