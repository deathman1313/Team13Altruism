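; BP_Ball is a physics ball that the BP_Teddy player knocks away by entering its Range component, letting it damage whatever it hits.
; On overlap, it enables mesh physics, applies a velocity-change impulse away from Teddy, and starts a one-time short timer to destroy itself.
; Hit events apply damage scaled by the hit component's linear speed, a calculation marked as not final.
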(event OnComponentBeginOverlap(Range)
  (params (OverlappedComponent :type Primitive%20Component%20Object%20Reference) (OtherActor :type Actor%20Object%20Reference) (OtherComp :type Primitive%20Component%20Object%20Reference) (OtherBodyIndex :type Integer) (bFromSweep :type Boolean) (SweepResult :type Hit%20Result%20Structure%20%28by%20ref%29))
  (bind _staticmesh (Variables|Default|GetStaticMesh))
  ;[1 1 1] Player Interaction
  (bind _asbp_teddy (Utilities|Casting|CastToBP_Teddy OtherActor))
  (Physics|SetSimulatePhysics _staticmesh true)
  (Physics|AddImpulse _staticmesh (* (Math|Vector|Normalize (- (Transformation|GetWorldLocation _staticmesh) (Transformation|GetWorldLocation (Variables|/Script/Engine.Character|GetCapsuleComponent _asbp_teddy)))) 1000) "None" true)
  ;[1 1 1] Destroy
  (Utilities|FlowControl|DoOnce false
    (:Completed
      (Utilities|Time|SetTimerbyEvent (delegate Custom|Destroy) 1.0))))

(event Custom|Destroy
  ;[1 1 1] Destroy
  (Actor|DestroyActor))

(event EventBeginPlay
  (|CallParentFunction) ; This node is disabled and will not be called.\nDrag off pins to build functionality.
)

(event Collision|EventActorBeginOverlap
  (params (OtherActor :type Actor%20Object%20Reference))
  (|CallParentFunction OtherActor) ; This node is disabled and will not be called.\nDrag off pins to build functionality.
)

(event EventTick
  (params (DeltaSeconds :type Float%20%28single-precision%29))
  (|CallParentFunction DeltaSeconds) ; This node is disabled and will not be called.\nDrag off pins to build functionality.
)

(event Collision|EventHit
  (params (MyComp :type Primitive%20Component%20Object%20Reference) (Other :type Actor%20Object%20Reference) (OtherComp :type Primitive%20Component%20Object%20Reference) (bSelfMoved :type Boolean) (HitLocation :type Vector :default "0, 0, 0") (HitNormal :type Vector :default "0, 0, 0") (NormalImpulse :type Vector :default "0, 0, 0") (Hit :type Hit%20Result%20Structure%20%28by%20ref%29))
  ;[1 1 1] Damage
  (bind _returnvalue (Physics|GetPhysicsLinearVelocity MyComp "None"))
  (Game|Damage|ApplyDamage Other (/ (Math|Vector|VectorLength _returnvalue) 1e+02) 0 self "/Script/Engine.DamageType"))

(fn ConstructionScript
  (|CallParentFunction))